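; Game instance Blueprint that persists the player's high score through a BP_Save save-game object.
; The Savescore event loads the existing save slot, or creates a new BP_Save seeded with the incoming score, then writes it back.
; For an existing save, the stored high score is replaced by the CompareScore result, whose graph holds nodes for selecting the larger score.
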(event `Save score`
  (params (Score :type Integer))
  (set `self.New score` Score)
  (bind _returnvalue (`GameplayStatics.DoesSaveGameExist` (`self.Save name`)))
  (if _returnvalue
    (bind _returnvalue_2 (`GameplayStatics.LoadGameFromSlot` (`self.Save name`)))
    (bind _asbp_save (cast `/Game/Blueprint/Save/BP_Save` _returnvalue_2))
    (bind _output_get (set `self.Save REF` _asbp_save))
    (set `/Game/Blueprint/Save/BP_Save.Highscore` (`self.Compare score` (`/Game/Blueprint/Save/BP_Save.Highscore` _output_get) (`self.New score`)) (`self.Save REF`))
    (else
      (bind _returnvalue_3 (`GameplayStatics.CreateSaveGameObject` "/Game/Blueprint/Save/BP_Save.BP_Save_C"))
      (bind _output_get_2 (set `self.Save REF` _returnvalue_3))
      (set `/Game/Blueprint/Save/BP_Save.Highscore` (`self.New score`) _output_get_2)))
  (`GameplayStatics.SaveGameToSlot` (`self.Save REF`) (`self.Save name`)))