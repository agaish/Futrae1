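; Obstacle with a pair of platforms, one randomly chosen at BeginPlay as a fake that falls.
; Extends a parent Blueprint, caching the second platform's starting transform alongside the inherited BeginPlay.
; The first player character overlapping either trigger box runs the same branch, calling Fall on the fake platform with its initial transform, whichever box was entered.
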(event `self.ReceiveBeginPlay`
  (`parent.ReceiveBeginPlay`)
  (set `self.Initial transform 2` (`SceneComponent.K2_GetComponentToWorld` (`self.Plateform2`)))
  (set `self.bIsLeftFake?` (`KismetMathLibrary.RandomBool`)))

(event `self.Box2.OnComponentBeginOverlap`
  (params (OverlappedComponent :type "PrimitiveComponent Object Reference") (OtherActor :type "Actor Object Reference") (OtherComp :type "PrimitiveComponent Object Reference") (OtherBodyIndex :type Integer) (bFromSweep :type Boolean) (SweepResult :type "HitResult Structure (by ref)"))
  (if (== OtherActor (`GameplayStatics.GetPlayerCharacter` 0))
    (if (`self.bIsLeftFake?`) :!label _label
      (`self.Fall` (`self.Plateform2`) (`self.Initial transform 2`))
      (else
        (`self.Fall` (`self.Plateform`) (`self.Initial transform`))))))

(event `self.Box.OnComponentBeginOverlap`
  (params (OverlappedComponent :type "PrimitiveComponent Object Reference") (OtherActor :type "Actor Object Reference") (OtherComp :type "PrimitiveComponent Object Reference") (OtherBodyIndex :type Integer) (bFromSweep :type Boolean) (SweepResult :type "HitResult Structure (by ref)"))
  (if (== OtherActor (`GameplayStatics.GetPlayerCharacter` 0))
    (goto _label)))

(fn `UserConstructionScript`
  (`parent.UserConstructionScript`))