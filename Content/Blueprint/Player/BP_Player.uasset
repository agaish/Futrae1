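; BP_Player is the player character, with Enhanced Input movement, camera look and jumping, plus modular body-part meshes and a score.
; The construction script makes the part meshes follow the main mesh via Leader Pose, and Equip swaps a part's skeletal mesh by type.
; NewScore adds to a clamped score and updates a HUD widget created at BeginPlay.
; Tab or the SaveGame event passes the score to GI_MyInstance for saving.
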(event `Key|Tab`
  (params (Key :type "Key Structure"))
  (:`Pressed`
    (bind _asgi_my_instance (cast `/Game/Blueprint/GI_MyInstance` (`GameplayStatics.GetGameInstance`) :!label _label))
    (`/Game/Blueprint/GI_MyInstance.Save score` _asgi_my_instance (`self.Score`))))

(event `/Game/Blueprint/Interface/BPI_Interactions.Save game`
  (goto _label))

(event `/Game/Blueprint/Interface/BPI_Interactions.New score`
  (params (Score :type Integer))
  (bind _output_get (set `self.Score` (`KismetMathLibrary.Clamp` (+ (`self.Score`) Score) 0 9999)))
  (`/Game/Blueprint/Widget/WP_Score.Score increase` (`self.HUD Score ref`) _output_get))

(event `self.ReceiveBeginPlay`
  (bind _returnvalue (`|CreateWidget` "/Game/Blueprint/Widget/WP_Score.WP_Score_C"))
  (bind _output_get (set `self.HUD Score ref` _returnvalue))
  (`UserWidget.AddToViewport` _output_get 0))

(event `EnhancedInput|/Game/Blueprint/Player/Input/IA_MoveForward`
  (params (ActionValue :type "Float (double-precision)") (ElapsedSeconds :type "Float (double-precision)") (TriggeredSeconds :type "Float (double-precision)") (InputAction :type "InputAction Object Reference" :default "/Game/Blueprint/Player/Input/IA_MoveForward.IA_MoveForward"))
  (bind (_returnvalue_roll _returnvalue_pitch _returnvalue_yaw) (`KismetMathLibrary.BreakRotator` (`self.GetControlRotation`)))
  (:`Triggered`
    (`self.AddMovementInput` (`KismetMathLibrary.GetForwardVector` (`KismetMathLibrary.MakeRotator` 0.0 0.0 _returnvalue_yaw)) ActionValue)))

(event `EnhancedInput|/Game/Blueprint/Player/Input/IA_MoveRight`
  (params (ActionValue :type "Float (double-precision)") (ElapsedSeconds :type "Float (double-precision)") (TriggeredSeconds :type "Float (double-precision)") (InputAction :type "InputAction Object Reference" :default "/Game/Blueprint/Player/Input/IA_MoveRight.IA_MoveRight"))
  (bind (_returnvalue_roll _returnvalue_pitch _returnvalue_yaw) (`KismetMathLibrary.BreakRotator` (`self.GetControlRotation`)))
  (:`Triggered`
    (`self.AddMovementInput` (`KismetMathLibrary.GetRightVector` (`KismetMathLibrary.MakeRotator` 0.0 0.0 _returnvalue_yaw)) ActionValue)))

(event `EnhancedInput|/Game/Blueprint/Player/Input/IA_Camera`
  (params (ActionValue :type "Vector2D Structure") (ElapsedSeconds :type "Float (double-precision)") (TriggeredSeconds :type "Float (double-precision)") (InputAction :type "InputAction Object Reference" :default "/Game/Blueprint/Player/Input/IA_Camera.IA_Camera"))
  (:`Triggered`
    (`self.AddControllerPitchInput` ActionValue_Y)
    (`self.AddControllerYawInput` ActionValue_X)))

(event `EnhancedInput|/Game/Blueprint/Player/Input/IA_Jump`
  (params (ActionValue :type Boolean) (ElapsedSeconds :type "Float (double-precision)") (TriggeredSeconds :type "Float (double-precision)") (InputAction :type "InputAction Object Reference" :default "/Game/Blueprint/Player/Input/IA_Jump.IA_Jump"))
  (:`Started`
    (`self.Jump`))
  (:`Completed`
    (`self.StopJumping`)))

(event `/Game/Blueprint/Interface/BPI_Interactions.Equip`
  (params (Mesh :type "SkeletalMesh Object Reference") (`Part type` :type "/Game/Blueprint/Enumerator/E_Parts Enum" :default "NewEnumerator0"))
  (`SkeletalMeshComponent.SetSkeletalMeshAsset` (select `/Game/Blueprint/Enumerator/E_Parts` `Part type` :`NewEnumerator0` (`self.Chest`) :`NewEnumerator1` (`self.Legs`) :`NewEnumerator2` (`self.Accessories`) :`NewEnumerator4` (`self.Hair`) :`NewEnumerator5` (`self.Beard`)) Mesh))

(fn `UserConstructionScript`
  (`SkinnedMeshComponent.SetLeaderPoseComponent` (`self.Accessories`) (`self.Mesh`) false false)
  (`SkinnedMeshComponent.SetLeaderPoseComponent` (`self.Hands`) (`self.Mesh`) false false)
  (`SkinnedMeshComponent.SetLeaderPoseComponent` (`self.Legs`) (`self.Mesh`) false false)
  (`SkinnedMeshComponent.SetLeaderPoseComponent` (`self.Chest`) (`self.Mesh`) false false)
  (`SkinnedMeshComponent.SetLeaderPoseComponent` (`self.Beard`) (`self.Mesh`) false false)
  (`SkinnedMeshComponent.SetLeaderPoseComponent` (`self.Hair`) (`self.Mesh`) false false))